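; Quest manager that tracks the active quests in the game.
; On BeginPlay it finds the quest event bus actor and binds to its take-quest event.
; AddQuest stores each quest uniquely and binds to its completion event, while RemoveQuest drops a quest and reports completion back through the bus.
; The TakeQuest and CompleteQuest functions are empty, and add and remove print debug messages.
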(event Custom|Add%20Quest
  (params (Quest :type BP%20Quest%20Object%20Reference))
  (Utilities|Array|AddUnique (Variables|Default|GetQuests) Quest)
  (EventDispatchers|BindEventtoOnCompleted Quest (EventDispatchers|CreateEvent :!event Custom|Remove%20Quest))
  (Development|PrintString "Added New Quest"))

(event Custom|Remove%20Quest
  (params (Quest :type BP%20Quest%20Object%20Reference))
  (Utilities|Array|RemoveItem (Variables|Default|GetQuests) Quest)
  (Default|CompleteQuest (Variables|Default|GetQuestEventBus) Quest)
  (Development|PrintString "Removed Completed Quest"))

(event EventBeginPlay
  (bind _returnvalue (Actor|GetActorOfClass "/Game/QuestSystem/BP_QuestEventBus.BP_QuestEventBus_C"))
  (Utilities|IsValid _returnvalue
    (:Is%20Valid
      (bind _output_get (Variables|Default|SetQuestEventBus _returnvalue))
      (EventDispatchers|BindEventtoOnTakeQuest _output_get (EventDispatchers|CreateEvent :!event Custom|Add%20Quest)))))

(fn ConstructionScript)

(fn TakeQuest
  (params (Quest :type BP%20Quest%20Object%20Reference)))

(fn CompleteQuest
  (params (Quest :type BP%20Quest%20Object%20Reference)))