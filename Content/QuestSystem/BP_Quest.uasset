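; BP_Quest is a quest object that tracks its own activation and completion state through a shared QuestChannel.
; On BeginPlay it binds to the channel's activated and completed events, and runs QuestActive if already in the active state.
; Incoming events apply only when UniqueID matches, updating State and calling QuestActive or QuestCompleted.
; Complete broadcasts the quest through the channel, so its own state change arrives via that event.
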(event Custom|QuestActiveEvent
  (params (Quest :type BP%20Quest%20Object%20Reference))
  (CallFunction|TryActivateQuest Quest))

(event Custom|QuestCompletedEvent
  (params (Quest :type BP%20Quest%20Object%20Reference))
  (CallFunction|TryCompleteQuest Quest))

(event EventBeginPlay
  (EventDispatchers|BindEventtoQuestActivatedEvent (Variables|Default|GetQuestChannel) (delegate Custom|QuestActiveEvent))
  (EventDispatchers|BindEventtoQuestCompleteEvent (Variables|Default|GetQuestChannel) (delegate Custom|QuestCompletedEvent))
  (if (Utilities|Enum|Equal(Enum) (Variables|Default|GetState) "NewEnumerator1")
    (CallFunction|QuestActive)))

(fn ConstructionScript)

(fn TryActivateQuest
  (params (ActivatedQuest :type BP%20Quest%20Object%20Reference))
  (if (Utilities|Enum|Equal(Enum) (Variables|BP_Quest_C|GetUniqueID ActivatedQuest) (Variables|Default|GetUniqueID))
    (Variables|Default|SetState "NewEnumerator1")
    (CallFunction|QuestActive)))

(fn TryCompleteQuest
  (params (self2 :type BP%20Quest%20Object%20Reference))
  (if (Utilities|Enum|Equal(Enum) (Variables|BP_Quest_C|GetUniqueID self2) (Variables|Default|GetUniqueID))
    (Variables|Default|SetState "NewEnumerator2")
    (CallFunction|QuestCompleted)))

(fn Complete
  (Default|CallQuestCompleteEvent (Variables|Default|GetQuestChannel) self))